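; BP_SplineBase is a spline actor that builds a chain of deforming static mesh segments along its path.
; The construction script adds one spline mesh per section length, optionally derived from the actor's X scale, with configurable mesh and collision.
; FullLengthSegments omits the shorter remainder segment at the end.
; Helper functions sample each segment's local endpoints by distance, clamping tangents to section length to suit the segment spacing.
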(event EventBeginPlay)

(event Collision|EventActorBeginOverlap
  (params (OtherActor :type Actor%20Object%20Reference)))

(event EventTick
  (params (DeltaSeconds :type Float%20%28single-precision%29)))

(fn ConstructionScript
  (if (Variables|Default|GetAllow%20Scaling)
    (Variables|Default|SetSection%20Length (* (.x (Transformation|GetActorScale3D)) 1e+02)))
  (if (Variables|Default|GetFullLength%20Segments)
    (for _index (range 0 (- (Math|Float|Truncate (/ (Spline|GetSplineLength (Variables|Default|GetSpline)) (Variables|Default|GetSection%20Length))) 1))
      (LocalVariables|SetIndex _index)
      (bind _returnvalue (AddComponent|AddSplineMeshComponent false))
      (Components|StaticMesh|SetStaticMesh _returnvalue (Variables|Default|GetSplineMesh))
      (SplineMesh|SetForwardAxis _returnvalue "X" true)
      (bind (_outgoing_position _outgoing_tangent) (CallFunction|GetStartPosTangent (LocalVariables|GetIndex)))
      (bind (_outgoing_position_2 _outgoing_tangent_2) (CallFunction|GetEndPosTangent (LocalVariables|GetIndex)))
      (SplineMesh|SetStartandEnd _returnvalue _outgoing_position _outgoing_tangent _outgoing_position_2 _outgoing_tangent_2 true :!class /Script/Engine.SplineMeshComponent)
      (Collision|SetCollisionEnabled _returnvalue (Variables|Default|GetCollisionType)))
    (else
      (for _index_2 (range 0 (Math|Float|Truncate (/ (Spline|GetSplineLength (Variables|Default|GetSpline)) (Variables|Default|GetSection%20Length))))
        (LocalVariables|SetIndex _index_2)
        (bind _returnvalue_2 (AddComponent|AddSplineMeshComponent false))
        (Components|StaticMesh|SetStaticMesh _returnvalue_2 (Variables|Default|GetSplineMesh))
        (SplineMesh|SetForwardAxis _returnvalue_2 "X" true)
        (bind (_outgoing_position_3 _outgoing_tangent_3) (CallFunction|GetStartPosTangent (LocalVariables|GetIndex)))
        (bind (_outgoing_position_4 _outgoing_tangent_4) (CallFunction|GetEndPosTangent (LocalVariables|GetIndex)))
        (SplineMesh|SetStartandEnd _returnvalue_2 _outgoing_position_3 _outgoing_tangent_3 _outgoing_position_4 _outgoing_tangent_4 true :!class /Script/Engine.SplineMeshComponent)
        (Collision|SetCollisionEnabled _returnvalue_2 (Variables|Default|GetCollisionType))))))

(fn GetStartPosTangent
  (params (Incoming%20Index :type Integer))
  (bind _spline (Variables|Default|GetSpline))
  (bind _section_length (Variables|Default|GetSection%20Length))
  (bind _returnvalue (* Incoming%20Index _section_length))
  (return (Spline|GetLocationatDistanceAlongSpline _spline _returnvalue "Local") (Math|Vector|ClampVectorSize (Spline|GetTangentatDistanceAlongSpline _spline _returnvalue "Local") 0.0 (Variables|Default|GetSection%20Length))))

(fn GetEndPosTangent
  (params (Incoming%20Index :type Integer))
  (bind _returnvalue (+ Incoming%20Index 1))
  (bind _spline (Variables|Default|GetSpline))
  (bind _section_length (Variables|Default|GetSection%20Length))
  (bind _returnvalue_2 (* _returnvalue _section_length))
  (return (Spline|GetLocationatDistanceAlongSpline _spline _returnvalue_2 "Local") (Math|Vector|ClampVectorSize (Spline|GetTangentatDistanceAlongSpline _spline _returnvalue_2 "Local") 0.0 (Variables|Default|GetSection%20Length))))
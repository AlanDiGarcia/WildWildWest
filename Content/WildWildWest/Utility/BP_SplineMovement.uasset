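; BP_SplineMovement is a utility Blueprint that drives a MineCart actor along a spline.
; The construction script snaps the cart to the spline's start point.
; On BeginPlay, a timeline at a rate of one over PlayRate plays, mapping its track to a distance between start and last spline point.
; Each update places the cart there in world space, rotated to face the spline tangent.
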(event EventBeginPlay
  (bind _spline (Variables|Default|GetSpline))
  (Utilities|FlowControl|Sequence
    (:then_0
      (Components|Timeline|SetPlayRate (Variables|Default|GetTimeline) (/ 1.0 (Variables|Default|GetPlay%20Rate))))
    (:then_1
      (bind _newtrack_0 (Timeline|Timeline Play)
        (:Update
          (Transformation|SetActorLocationAndRotation (Variables|Default|GetMine%20Cart) (Spline|GetLocationatDistanceAlongSpline (Variables|Default|GetSpline) (Math|Float|Lerp 0.0 (Spline|GetDistanceAlongSplineatSplinePoint _spline (- (Spline|GetNumberOfSplinePoints _spline) 1)) _newtrack_0) "World") (Math|Conversions|RotationFromXVector (Spline|GetTangentatDistanceAlongSpline (Variables|Default|GetSpline) (Math|Float|Lerp 0.0 (Spline|GetDistanceAlongSplineatSplinePoint _spline (- (Spline|GetNumberOfSplinePoints _spline) 1)) _newtrack_0) "World"))))))))

(fn ConstructionScript
  (Transformation|SetActorLocation (Variables|Default|GetMine%20Cart) (Spline|GetLocationatDistanceAlongSpline (Variables|Default|GetSpline) 0.0 "World") false false))
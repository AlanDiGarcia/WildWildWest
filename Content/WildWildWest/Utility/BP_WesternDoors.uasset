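; BP_WesternDoors is a pair of Western-style doors that make a wooden thud when something enters their trigger boxes.
; On BeginPlay, it locks the left and right cylinder components to XY-plane constraint mode, restricting their physics movement to horizontal.
; Each side's box overlap plays the same dull wood sound at that door's location, with no filtering on the overlapping actor.
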(event OnComponentBeginOverlap(RightBox)
  (params (OverlappedComponent :type Primitive%20Component%20Object%20Reference) (OtherActor :type Actor%20Object%20Reference) (OtherComp :type Primitive%20Component%20Object%20Reference) (OtherBodyIndex :type Integer) (bFromSweep :type Boolean) (SweepResult :type Hit%20Result%20Structure%20%28by%20ref%29))
  (Audio|PlaySoundatLocation "/Game/WildWildWest/Audio/SoundCues/WoodDullHardCue.WoodDullHardCue" (Transformation|GetWorldLocation (Variables|Default|GetRight%20Door)) "0, 0, 0" 1.0 1.0 0.0 0 0 0 0))

(event OnComponentBeginOverlap(LeftBox)
  (params (OverlappedComponent :type Primitive%20Component%20Object%20Reference) (OtherActor :type Actor%20Object%20Reference) (OtherComp :type Primitive%20Component%20Object%20Reference) (OtherBodyIndex :type Integer) (bFromSweep :type Boolean) (SweepResult :type Hit%20Result%20Structure%20%28by%20ref%29))
  (Audio|PlaySoundatLocation "/Game/WildWildWest/Audio/SoundCues/WoodDullHardCue.WoodDullHardCue" (Transformation|GetWorldLocation (Variables|Default|GetLeft%20Door)) "0, 0, 0" 1.0 1.0 0.0 0 0 0 0))

(event EventBeginPlay
  (Class|PrimitiveComponent|SetConstraintMode (Variables|Default|GetLeft%20Cylinder) "XYPlane")
  (Class|PrimitiveComponent|SetConstraintMode (Variables|Default|GetRight%20Cylinder) "XYPlane"))

(fn ConstructionScript)
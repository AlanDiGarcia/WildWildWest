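; BP_Bottle is a Wild West obstacle prop that makes a glass sound when something overlaps it.
; The construction script randomly picks one of two bottle meshes for visual variety.
; A capsule overlap plays either a glass or glass-shatter cue at the mesh location, each with equal odds.
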(event OnComponentBeginOverlap(Capsule)
  (params (OverlappedComponent :type Primitive%20Component%20Object%20Reference) (OtherActor :type Actor%20Object%20Reference) (OtherComp :type Primitive%20Component%20Object%20Reference) (OtherBodyIndex :type Integer) (bFromSweep :type Boolean) (SweepResult :type Hit%20Result%20Structure%20%28by%20ref%29))
  (bind _staticmesh (Variables|Default|GetStaticMesh))
  (bind _returnvalue (Transformation|GetWorldLocation _staticmesh))
  (if (Math|Random|RandomBoolwithWeight 0.5)
    (Audio|PlaySoundatLocation "/Game/WildWildWest/Audio/SoundCues/GlassCue.GlassCue" _returnvalue "0, 0, 0" 1.0 1.0 0.0 0 0 0 0)
    (else
      (Audio|PlaySoundatLocation "/Game/WildWildWest/Audio/SoundCues/GlassShatterCue.GlassShatterCue" _returnvalue "0, 0, 0" 1.0 1.0 0.0 0 0 0 0))))

(fn ConstructionScript
  (if (Math|Random|RandomBoolwithWeight 0.5)
    (Components|StaticMesh|SetStaticMesh (Variables|Default|GetStaticMesh) "/Game/WildWildWest/SM/SM_Bottle1.SM_Bottle1")
    (else
      (Components|StaticMesh|SetStaticMesh (Variables|Default|GetStaticMesh) "/Game/WildWildWest/SM/SM_Bottle2.SM_Bottle2"))))
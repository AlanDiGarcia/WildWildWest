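; BP_Can is a can obstacle in the Wild Wild West game that varies its look and makes a metallic noise when touched.
; The construction script gives its static mesh a random material from the first four entries of a material list.
; Any overlap with its capsule plays one of two metal sound cues at the mesh location, chosen with even odds.
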(event OnComponentBeginOverlap(Capsule)
  (params (OverlappedComponent :type Primitive%20Component%20Object%20Reference) (OtherActor :type Actor%20Object%20Reference) (OtherComp :type Primitive%20Component%20Object%20Reference) (OtherBodyIndex :type Integer) (bFromSweep :type Boolean) (SweepResult :type Hit%20Result%20Structure%20%28by%20ref%29))
  (bind _staticmesh (Variables|Default|GetStaticMesh))
  (bind _returnvalue (Transformation|GetWorldLocation _staticmesh))
  (if (Math|Random|RandomBoolwithWeight 0.5)
    (Audio|PlaySoundatLocation "/Game/WildWildWest/Audio/SoundCues/MetalDropCue.MetalDropCue" _returnvalue "0, 0, 0" 1.0 1.0 0.0 0 0 0 0)
    (else
      (Audio|PlaySoundatLocation "/Game/WildWildWest/Audio/SoundCues/MetalHighCue.MetalHighCue" _returnvalue "0, 0, 0" 1.0 1.0 0.0 0 0 0 0))))

(fn ConstructionScript
  (Rendering|Material|SetMaterial (Variables|Default|GetStaticMesh) 0 (Utilities|Array|Get(acopy) (Variables|Default|GetMaterialList) (Math|Random|RandomIntegerinRange 0 3))))
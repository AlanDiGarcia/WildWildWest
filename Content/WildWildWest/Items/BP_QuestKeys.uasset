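; BP_QuestKeys is a quest item that the tumbleweed picks up and hands over to the shopkeeper.
; On the first sphere overlap with BP_Tumbleweed, it snaps to the tumbleweed's ItemPoint2 and stores the attach result in KeysAttached.
; The Detach event runs a timeline that lerps the keys from that item point to the BP_Shopkeeper's mesh with sweep on, then destroys the actor.
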(event OnComponentBeginOverlap(Sphere)
  (params (OverlappedComponent :type Primitive%20Component%20Object%20Reference) (OtherActor :type Actor%20Object%20Reference) (OtherComp :type Primitive%20Component%20Object%20Reference) (OtherBodyIndex :type Integer) (bFromSweep :type Boolean) (SweepResult :type Hit%20Result%20Structure%20%28by%20ref%29))
  (bind _asbp_tumbleweed (Utilities|Casting|CastToBP_Tumbleweed OtherActor))
  (Utilities|FlowControl|DoOnce false
    (:Completed
      (Utilities|FlowControl|Sequence
        (:then_0
          (bind _returnvalue (Transformation|AttachComponentToComponent (Variables|/Game/WildWildWest/Player/BP_Tumbleweed.BP_Tumbleweed_C|GetItemPoint2 _asbp_tumbleweed) "None" "SnapToTarget" "SnapToTarget" "KeepRelative" true)))
        (:then_1
          (Variables|/Game/WildWildWest/Player/BP_Tumbleweed.BP_Tumbleweed_C|SetKeys%20Attached _asbp_tumbleweed _returnvalue))))))

(event Custom|Detach
  (params (Incoming%20Tumbleweed :type BP%20Tumbleweed%20Object%20Reference))
  (bind _returnvalue (Actor|GetActorOfClass "/Game/WildWildWest/NPC/BP_Shopkeeper.BP_Shopkeeper_C"))
  (bind _newtrack_0 (Timeline|Timeline_0 Play)
    (:Update
      (Transformation|SetWorldLocation (Variables|Default|GetDefaultSceneRoot) (Math|Vector|Lerp(Vector) (Transformation|GetWorldLocation (Variables|/Game/WildWildWest/Player/BP_Tumbleweed.BP_Tumbleweed_C|GetItemPoint2 Incoming%20Tumbleweed)) (Transformation|GetWorldLocation (Variables|/Game/WildWildWest/NPC/BP_Shopkeeper.BP_Shopkeeper_C|GetStaticMesh _returnvalue)) _newtrack_0) true false))
    (:Finished
      (Actor|DestroyActor))))

(fn ConstructionScript
  (|CallParentFunction))
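; BP_GunSheriff is a pickup gun in WildWildWest that attaches to a tumbleweed and fires sheriff bullets.
; When its Sphere overlaps a BP_Tumbleweed, it snaps onto that actor's GunPoint in location and rotation, keeping relative scale.
; The Shooting event spawns a BP_BulletSheriff at the Cube's location and rotation, then launches it along the Cube's negative right vector with a velocity-change impulse.
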(event OnComponentBeginOverlap(Sphere)
  (params (OverlappedComponent :type Primitive%20Component%20Object%20Reference) (OtherActor :type Actor%20Object%20Reference) (OtherComp :type Primitive%20Component%20Object%20Reference) (OtherBodyIndex :type Integer) (bFromSweep :type Boolean) (SweepResult :type Hit%20Result%20Structure%20%28by%20ref%29))
  (bind _asbp_tumbleweed (Utilities|Casting|CastToBP_Tumbleweed OtherActor))
  (Transformation|AttachComponentToComponent (Variables|/Game/WildWildWest/Player/BP_Tumbleweed.BP_Tumbleweed_C|GetGunPoint _asbp_tumbleweed) "None" "SnapToTarget" "SnapToTarget" "KeepRelative" true))

(event EventShooting
  (params (Incoming%20Control%20Rotation :type Rotator :default "0, 0, 0"))
  (bind _cube (Variables|Default|GetCube))
  (bind _returnvalue (Game|SpawnActorfromClass "/Game/WildWildWest/Items/BP_BulletSheriff.BP_BulletSheriff_C" (Math|Transform|MakeTransform (Transformation|GetWorldLocation _cube) (Transformation|GetWorldRotation _cube) "1.000000,1.000000,1.000000") "Undefined" "MultiplyWithRoot" 0 0))
  (Physics|AddImpulse (Variables|/Game/WildWildWest/Items/BP_BulletSheriff.BP_BulletSheriff_C|GetSphere _returnvalue) (* (Math|Vector|GetRightVector _cube) -3e+03) "None" true))

(fn ConstructionScript)